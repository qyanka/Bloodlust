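; BP_SaveManager handles checkpoint saving and loading for Bloodlust through one fixed save slot.
; ReadFromSlot loads and casts the BP_SaveGame, or creates a fresh one reporting success when none exists.
; SaveCheckpoint writes the given transform with placeholder checkpoint ID and level name, then saves via WriteToSlot.
; GetLastCheckpointTransform returns the stored transform and read success, which is also true for a new, unsaved object.
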(event EventBeginPlay)

(event Collision|EventActorBeginOverlap
  (params (OtherActor :type Actor%20Object%20Reference)))

(event EventTick
  (params (DeltaSeconds :type Float%20%28single-precision%29)))

(fn ConstructionScript)

(fn WritetoSlot
  (params (SaveObject%20%20 :type BP%20Save%20Game%20Object%20Reference))
  (bind _returnvalue (SaveGame|SaveGametoSlot SaveObject%20%20 "BloodlustSave"))
  (return _returnvalue))

(fn ReadfromSlot
  (bind _returnvalue (SaveGame|DoesSaveGameExist "BloodlustSave"))
  (if _returnvalue
    (bind _returnvalue_2 (SaveGame|LoadGamefromSlot "BloodlustSave"))
    (bind _asbp_save_game (Utilities|Casting|CastToBP_SaveGame _returnvalue_2)
      (:then
        (return _asbp_save_game true))
      (:CastFailed
        (return _asbp_save_game false)))
    (else
      (bind _returnvalue_3 (SaveGame|CreateSaveGameObject "/Game/Bloodlust/Core/SaveSystem/BP_SaveGame.BP_SaveGame_C"))
      (return _returnvalue_3 true))))

(fn SaveCheckpoint
  (params (NewTransform :type Transform))
  (bind _saveobject_ (CallFunction|ReadfromSlot))
  (bind _output_get (LocalVariables|SetSaveObject _saveobject_))
  ;[0.15 0.15 0.15 0.5] CheckpointID&LastLevelName TBD
  (Variables|/Game/Bloodlust/Core/SaveSystem/BP_SaveGame.BP_SaveGame_C|SetSaveData%20%20 _output_get (Utilities|Struct|MakeST_SaveData NewTransform "DefaultCheckpoint" "None"))
  (CallFunction|WritetoSlot (LocalVariables|GetSaveObject)))

(fn GetLastCheckpointTransform
  (bind (_saveobject_ _success) (CallFunction|ReadfromSlot))
  (return (.playertransform (Variables|/Game/Bloodlust/Core/SaveSystem/BP_SaveGame.BP_SaveGame_C|GetSaveData%20%20 _saveobject_)) _success))