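; Bloodlust game instance that holds key-collection progress and capsule activation state.
; AddKey increments the collected count and broadcasts OnKeyCollected with the new total.
; IsCapsuleReady compares that count to the required key count, while simple accessors expose the counts and set the activated flag.
; ResetKeys clears both the count and the capsule flag.
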(fn AddKey
  (bind _result (Math|Integer|IncrementInt (Variables|Default|GetKeysCollected))
    (:%20%20
      (bind _output_get (Variables|Default|SetKeysCollected _result))
      (Default|CallOnKeyCollected _output_get))))

(fn ResetKeys
  (Variables|Default|SetKeysCollected 0)
  (Variables|Default|SetbCapsuleActivated%20 false))

(fn IsCapsuleReady
  (if (>= (Variables|Default|GetKeysCollected) (Variables|Default|GetRequiredKeysCount))
    (return true)))

(fn GetKeysCollected
  (return (Variables|Default|GetKeysCollected)))

(fn SetKeysCollected
  (params (KeysCollected :type Integer))
  (Variables|Default|SetKeysCollected KeysCollected))

(fn GetRecuiredKeysCount
  (return (Variables|Default|GetRequiredKeysCount)))

(fn SetCapsuleActivated
  (Variables|Default|SetbCapsuleActivated%20 true))