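; Player controller for Bloodlust that creates the crosshair and interaction prompt widgets and maps Enhanced Input to the possessed BP_PlayerCharacter.
; Handles movement, look, jump, crouch and sprint, forwarding aim and shoot to the WeaponComponent.
; Movement, crouch, interact and shoot actions report noise to the character's NoiseComponent, named from state flags.
; A looping timer line-traces from the follow camera, caching nearby BPI_Interactable actors for the prompt and interact input.
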(event Custom|TraceForInteractables
  (bind _interactionwidget (Variables|Default|GetInteractionWidget))
  ;[0.15 0.15 0.15 0.5] Interaction trace
  (bind _outhit (CallFunction|PlayerTrace 6e+02 "None" "(R=0.363120,G=1.000000,B=0.000000,A=1.000000)"))
  (Utilities|IsValid (.HitActor (Collision|BreakHitResult _outhit))
    (:Is%20Valid
      (if (Utilities|DoesObjectImplementInterface (.HitActor (Collision|BreakHitResult _outhit)) "/Game/Bloodlust/Interfaces/BPI_Interactable.BPI_Interactable_C")
        (if (< (.Distance (Collision|BreakHitResult _outhit)) 2e+02)
          (Development|PrintString (Utilities|String|Append "Current interactable" (Utilities|GetDisplayName (.HitActor (Collision|BreakHitResult _outhit)))))
          (bind _output_get (Variables|Default|SetCurrentInteractable (.HitActor (Collision|BreakHitResult _outhit))))
          (bind _text (Class|BPIInteractable|GetInteractionText(Message) _output_get))
          (Default|SetPromptText _interactionwidget _text)
          (Widget|SetVisibility _interactionwidget "Visible")
          (else
            (Widget|SetVisibility _interactionwidget "Hidden" :!label _label)
            (Variables|Default|SetCurrentInteractable 0)))
        (else
          (goto _label))))
    (:Is%20Not%20Valid
      (goto _label))))

(event Input|EnhancedActionEvents|EnhancedInputActionIA_Crouch
  (params (ActionValue :type Boolean) (ElapsedSeconds :type Float%20%28double-precision%29) (TriggeredSeconds :type Float%20%28double-precision%29) (InputAction :type Input%20Action%20Object%20Reference :default "/Game/Bloodlust/Core/EnhancedInput/Actions/IA_Crouch.IA_Crouch"))
  (bind _playercharacter (Variables|Default|GetPlayerCharacter))
  ;[0.15 0.15 0.15 0.5] Crouch
  (:Started
    (Variables|Default|SetbIsCroushing true)
    (bind _actionname (CallFunction|GetNoiseActorName))
    (Default|Noise (Variables|Default|GetNoise%20Component) _actionname (Transformation|GetSocketLocation (Variables|/Script/Engine.Character|GetCapsuleComponent _playercharacter) "None"))
    (if (Variables|/Script/Engine.Character|GetbIsCrouched _playercharacter)
      (Character|UnCrouch _playercharacter)
      (else
        (Character|Crouch _playercharacter))))
  (:Completed
    (Variables|Default|SetbIsCroushing false)))

(event Input|EnhancedActionEvents|EnhancedInputActionIA_Sprint
  (params (ActionValue :type Boolean) (ElapsedSeconds :type Float%20%28double-precision%29) (TriggeredSeconds :type Float%20%28double-precision%29) (InputAction :type Input%20Action%20Object%20Reference :default "/Game/Bloodlust/Core/EnhancedInput/Actions/IA_Sprint.IA_Sprint"))
  (bind _movementcomponent (Variables|Default|GetMovementComponent))
  ;[0.15 0.15 0.15 0.5] Run
  (:Triggered
    (bind _actionname (CallFunction|GetNoiseActorName))
    (Default|Noise (Variables|Default|GetNoise%20Component) _actionname (Transformation|GetWorldLocation (Variables|/Script/Engine.Character|GetCapsuleComponent (Variables|Default|GetPlayerCharacter))))
    (Variables|/Script/Engine.CharacterMovementComponent|SetMaxWalkSpeed _movementcomponent 8.5e+02))
  (:Completed
    (Variables|/Script/Engine.CharacterMovementComponent|SetMaxWalkSpeed _movementcomponent 6e+02)))

(event Input|EnhancedActionEvents|EnhancedInputActionIA_Move
  (params (ActionValue :type Vector%202D%20Structure) (ElapsedSeconds :type Float%20%28double-precision%29) (TriggeredSeconds :type Float%20%28double-precision%29) (InputAction :type Input%20Action%20Object%20Reference :default "/Game/Bloodlust/Core/EnhancedInput/Actions/IA_Move.IA_Move"))
  (bind _returnvalue (Pawn|GetControlRotation :!class /Script/Engine.Controller))
  ;[0.15 0.15 0.15 0.5] Walk WASD
  (:Triggered
    (Variables|Default|SetbIsWalking true)
    (bind _actionname (CallFunction|GetNoiseActorName))
    (Default|Noise (Variables|Default|GetNoise%20Component) _actionname (Transformation|GetWorldLocation (Variables|/Script/Engine.Character|GetCapsuleComponent (Variables|Default|GetPlayerCharacter))))
    (bind _movementcomponent (Variables|Default|GetMovementComponent)
      (:then
        (Utilities|FlowControl|Sequence
          (:then_0
            ;;[0.15 0.15 0.15 0.5] Forward(Yaw)
            (Class|PawnMovementComponent|AddInputVector _movementcomponent (* (.y ActionValue) (Math|Vector|GetForwardVector (Math|Rotator|MakeRotator 0.0 0.0 (.yaw (Pawn|GetControlRotation :!class /Script/Engine.Controller))))) false))
          (:then_1
            ;;[0.15 0.15 0.15 0.5] Right(roll/yaw)
            (Class|PawnMovementComponent|AddInputVector _movementcomponent (* (.x ActionValue) (Math|Vector|GetRightVector (Math|Rotator|MakeRotator (.roll _returnvalue) 0.0 (.yaw _returnvalue)))) false))))
      (:else)))
  (:Completed
    (Variables|Default|SetbIsWalking false)
    (Development|PrintString "walk false")))

(event Input|EnhancedActionEvents|EnhancedInputActionIA_Look
  (params (ActionValue :type Vector%202D%20Structure) (ElapsedSeconds :type Float%20%28double-precision%29) (TriggeredSeconds :type Float%20%28double-precision%29) (InputAction :type Input%20Action%20Object%20Reference :default "/Game/Bloodlust/Core/EnhancedInput/Actions/IA_Look.IA_Look"))
  ;[0.15 0.15 0.15 0.5] Mouse Turn
  (Class|PlayerController|AddYawInput (.x ActionValue))
  (Class|PlayerController|AddPitchInput (.y ActionValue)))

(event Input|EnhancedActionEvents|EnhancedInputActionIA_Jump
  (params (ActionValue :type Boolean) (ElapsedSeconds :type Float%20%28double-precision%29) (TriggeredSeconds :type Float%20%28double-precision%29) (InputAction :type Input%20Action%20Object%20Reference :default "/Game/Bloodlust/Core/EnhancedInput/Actions/IA_Jump.IA_Jump"))
  (bind _playercharacter (Variables|Default|GetPlayerCharacter))
  ;[0.15 0.15 0.15 0.5] Jump takes a Character; BP’s a controller, so you gotta explicitly pass DodgeCharacter — cast’s done earlier
  (:Triggered
    (Character|Jump _playercharacter))
  (:Completed
    (Character|StopJumping _playercharacter)))

(event Input|EnhancedActionEvents|EnhancedInputActionIA_Aim
  (params (ActionValue :type Boolean) (ElapsedSeconds :type Float%20%28double-precision%29) (TriggeredSeconds :type Float%20%28double-precision%29) (InputAction :type Input%20Action%20Object%20Reference :default "/Game/Bloodlust/Core/EnhancedInput/Actions/IA_Aim.IA_Aim"))
  (bind _playercharacter (Variables|Default|GetPlayerCharacter))
  (bind _weaponcomponent (Variables|/Game/Bloodlust/Characters/Player/BP_PlayerCharacter.BP_PlayerCharacter_C|GetWeaponComponent _playercharacter))
  ;[0.15 0.15 0.15 0.5] Aim
  (:Started
    (Default|StartAiming _weaponcomponent))
  (:Completed
    (Default|StopAiming _weaponcomponent)))

(event Input|EnhancedActionEvents|EnhancedInputActionIA_Shoot
  (params (ActionValue :type Boolean) (ElapsedSeconds :type Float%20%28double-precision%29) (TriggeredSeconds :type Float%20%28double-precision%29) (InputAction :type Input%20Action%20Object%20Reference :default "/Game/Bloodlust/Core/EnhancedInput/Actions/IA_Shoot.IA_Shoot"))
  (bind _playercharacter (Variables|Default|GetPlayerCharacter))
  ;[0.15 0.15 0.15 0.5] Shoot
  (Variables|Default|SetbIsShooting true)
  (bind _actionname (CallFunction|GetNoiseActorName))
  (Default|Noise (Variables|Default|GetNoise%20Component) _actionname (Transformation|GetWorldLocation (Variables|/Script/Engine.Character|GetCapsuleComponent _playercharacter)))
  (Default|Shoot (Variables|/Game/Bloodlust/Characters/Player/BP_PlayerCharacter.BP_PlayerCharacter_C|GetWeaponComponent _playercharacter)))

(event Input|EnhancedActionEvents|EnhancedInputActionIA_Interact
  (params (ActionValue :type Boolean) (ElapsedSeconds :type Float%20%28double-precision%29) (TriggeredSeconds :type Float%20%28double-precision%29) (InputAction :type Input%20Action%20Object%20Reference :default "/Game/Bloodlust/Core/EnhancedInput/Actions/IA_Interact.IA_Interact"))
  ;[0.15 0.15 0.15 0.5] Interact
  (:Started
    (Variables|Default|SetbIsInteructing true)
    (bind _actionname (CallFunction|GetNoiseActorName))
    (Default|Noise (Variables|Default|GetNoise%20Component) _actionname (Transformation|GetWorldLocation (Variables|/Script/Engine.Character|GetCapsuleComponent (Variables|Default|GetPlayerCharacter))))
    (bind _currentinteractable (Variables|Default|GetCurrentInteractable)
      (:then
        (Class|BPIInteractable|Interact(Message) _currentinteractable _currentinteractable))
      (:else)))
  (:Completed
    (Variables|Default|SetbIsInteructing false)))

(event EventBeginPlay
  (bind _self self)
  (Utilities|FlowControl|Sequence
    (:then_0
      (bind _returnvalue (UserInterface|CreateWidget "/Game/Bloodlust/UI/WBP_InteractioinPrompt.WBP_InteractioinPrompt_C"))
      (bind _output_get (Variables|Default|SetInteractionWidget _returnvalue))
      (UserInterface|Viewport|AddtoViewport _output_get 0)
      (Widget|SetVisibility _output_get "Hidden"))
    (:then_1
      (bind _returnvalue_2 (UserInterface|CreateWidget "/Game/Bloodlust/UI/WBP_Crosshair.WBP_Crosshair_C"))
      (UserInterface|Viewport|AddtoViewport _returnvalue_2 0))
    (:then_2
      (Utilities|Time|SetTimerbyFunctionName 0 "TraceForInteractables" 0.3 true))
    (:then_3
      (Input|SetInputModeGameOnly _self false)
      (Variables|Default|SetbShowMouseCursor _self false)
      (Input|AddMappingContext (PlayerController|LocalPlayerSubsystems|GetEnhancedInputLocalPlayerSubsystem) "/Game/Bloodlust/Core/EnhancedInput/IMC_BloodDefault.IMC_BloodDefault" 0 "(bIgnoreAllPressedKeysUntilRelease=True,bForceImmediately=False,bNotifyUserSettings=False)")
      ;[0.15 0.15 0.15 0.5] PlayerController doesn’t own CharacterMovementComponent but has access to Pawn; if it's not a Character, Cast<ACharacter>() returns nullptr in C++ or Cast Failed in BP — recommended check the type before casting
      (bind _asbp_player_character (Utilities|Casting|CastToBP_PlayerCharacter (Pawn|GetControlledPawn)))
      (bind _output_get_2 (Variables|Default|SetPlayerCharacter _asbp_player_character))
      (Variables|Default|SetMovementComponent (Variables|/Script/Engine.Character|GetCharacterMovement _output_get_2))
      (Variables|Default|SetNoise%20Component (Variables|/Game/Bloodlust/Characters/Player/BP_PlayerCharacter.BP_PlayerCharacter_C|GetNoiseComponent _output_get_2)))))

(fn ConstructionScript)

(fn PlayerTrace
  (params (TraceLength :type Float%20%28double-precision%29) (DrawDebugType :type EDrawDebugTrace%20Enum :default "None") (TraceColor :type Linear%20Color%20Structure) (TraceHitColor :type Linear%20Color%20Structure))
  (bind (_start _end) (Utilities|TraceStartEndCalc TraceLength))
  (bind _outhit (Collision|LineTraceByChannel _start _end "TraceTypeQuery1" false 0 DrawDebugType true TraceColor TraceHitColor))
  (return _outhit))

(fn GetNoiseActorName
  (if (Variables|Default|GetbIsWalking)
    (Development|PrintString "walk")
    (elif (Variables|Default|GetbIsRunning)
      (Development|PrintString "run")
      (return "Run")
      (elif (Variables|Default|GetbIsCroushing)
        (Development|PrintString "crouch")
        (return "CrouchWalk")
        (elif (Variables|Default|GetbIsShooting)
          (Development|PrintString "shoot")
          (return "Shoot")
          (elif (Variables|Default|GetbIsInteructing)
            (Development|PrintString "interuct")
            (return "Interuct")
            (elif (and (Variables|Default|GetbIsWalking) (Variables|Default|GetbIsShooting))
              (Development|PrintString "walkshoot")
              (return "WalkShoot")
              (elif (and (Variables|Default|GetbIsRunning) (Variables|Default|GetbIsShooting))
                (Development|PrintString "runshoot")
                (return "RunShoot")
                (elif (and (Variables|Default|GetbIsCroushing) (Variables|Default|GetbIsShooting))
                  (Development|PrintString "crouchshoot")
                  (return "CrouchShoot")
                  (elif (and (Variables|Default|GetbIsCroushing) (Variables|Default|GetbIsInteructing))
                    (Development|PrintString "crouchinteruct")
                    (return "CrouchInteruct")
                    (else
                      (return "Idle"))))))))))))