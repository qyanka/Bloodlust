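; BP_Mirror is an interactable mirror for the Sonic Mirror puzzle, laid out mostly as stubs.
; Interact calls RotateMirror when CanInteract reports that the mirror is not already being interacted with.
; RotateMirror, OnMouseDrag and GetReflection, which takes incoming and outgoing traces, have no logic yet.
; The interaction text is empty and the highlight function only returns false.
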(event Custom|OnMouseDrag)

(event Custom|GetReflection
  (params (TraceIn :type Vector) (TraceOut :type Vector)))

(event Custom|RotateMirror)

(event EventInteract
  (params (Interactor :type Actor%20Object%20Reference))
  (CallFunction|CanInteract)
  (if true
    (CallFunction|RotateMirror)))

(fn ConstructionScript)

(fn CanInteract
  (return (not (Variables|Default|GetbIsInteracting%20))))

(fn GetInteractionText
  (return ""))

(fn SetHighlited
  (params (bIsHighlited :type Boolean))
  (return false))