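; T-shaped pipe piece for the Bloodflow puzzle, a child Blueprint that defines which sides connect at each rotation.
; UpdateConnectionDirs maps CurrentRotation to a four-entry boolean ConnectionDirs array with three open sides and one closed side that shifts with each step.
; It prints the rotation for debugging and reports out-of-range values as a bad rotation.
; The construction script only calls the parent.
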(event EventUpdateConnectionDirs
  (bind _currentrotation_ (Variables|Default|GetCurrentRotation%20))
  (Development|PrintString (Utilities|String|ToString(Integer) _currentrotation_) true true "(R=1.000000,G=0.947440,B=0.000000,A=1.000000)")
  (switch int _currentrotation_
    (:Default
      (Development|PrintString "BadRotation"))
    (:0
      (Variables|Default|SetConnectionDirs (Utilities|Array|MakeArray true true true false)))
    (:1
      (Variables|Default|SetConnectionDirs (Utilities|Array|MakeArray true true false true)))
    (:2
      (Variables|Default|SetConnectionDirs (Utilities|Array|MakeArray true false true true)))
    (:3
      (Variables|Default|SetConnectionDirs (Utilities|Array|MakeArray false true true true)))))

(fn ConstructionScript
  (|CallParentFunction))