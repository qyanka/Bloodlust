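; BP_Pipe_Cap is a single-opening end piece for the Bloodflow pipe puzzle in Bloodlust.
; It implements the UpdateConnectionDirs event, mapping each of the four CurrentRotation steps to a ConnectionDirs array with exactly one open side.
; An unrecognized rotation only prints a debug warning, and the construction script simply defers to its parent.
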(event EventUpdateConnectionDirs
  (switch int (Variables|Default|GetCurrentRotation%20)
    (:Default
      (Development|PrintString "BadRotation"))
    (:0
      (Variables|Default|SetConnectionDirs (Utilities|Array|MakeArray true false false false)))
    (:1
      (Variables|Default|SetConnectionDirs (Utilities|Array|MakeArray false false false true)))
    (:2
      (Variables|Default|SetConnectionDirs (Utilities|Array|MakeArray false false true false)))
    (:3
      (Variables|Default|SetConnectionDirs (Utilities|Array|MakeArray false true false false)))))

(fn ConstructionScript
  (|CallParentFunction))