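; L-shaped corner pipe piece for the Bloodflow puzzle, defining which sides are open at each rotation.
; UpdateConnectionDirs switches on CurrentRotation and sets the four-entry ConnectionDirs boolean array to one of four adjacent-side pairs.
; An out-of-range rotation only prints a "BadRotation" message.
; The construction script just calls the parent, and no other logic is defined here.
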(event EventUpdateConnectionDirs
  (switch int (Variables|Default|GetCurrentRotation%20)
    (:Default
      (Development|PrintString "BadRotation"))
    (:0
      (Variables|Default|SetConnectionDirs (Utilities|Array|MakeArray true true false false)))
    (:1
      (Variables|Default|SetConnectionDirs (Utilities|Array|MakeArray false true true false)))
    (:2
      (Variables|Default|SetConnectionDirs (Utilities|Array|MakeArray false false true true)))
    (:3
      (Variables|Default|SetConnectionDirs (Utilities|Array|MakeArray true false false true)))))

(fn ConstructionScript
  (|CallParentFunction))