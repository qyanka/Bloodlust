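; Base interactable pipe for the bloodflow puzzle, turning 90 degrees in yaw per interaction.
; A timeline animates the mesh, then updates CurrentRotation and calls the empty UpdateConnectionDirs hook, with IsRotating blocking input until shortly afterwards.
; Interact calls CheckFlow on BP_BloodflowManager right after starting the rotation, so the check runs before the connection update.
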(event Custom|RotatePipe
  (Variables|Default|SetbIsRotating true)
  (bind _output_get (Variables|Default|SetStartRotation (.yaw (Transformation|GetWorldRotation (Variables|Default|GetStaticMesh)))))
  (bind _newtrack_0 (Timeline|Timeline PlayFromStart)
    (:Update
      (Transformation|SetWorldRotation (Variables|Default|GetStaticMesh) (Math|Rotator|MakeRotator 0.0 0.0 (Math|Float|Lerp (Variables|Default|GetStartRotation) (Math|Float|%(Float) (+ _output_get 9e+01) 3.6e+02) _newtrack_0)) false false))
    (:Finished
      (Variables|Default|SetCurrentRotation%20 (Math|Integer|%(Integer) (+ (Variables|Default|GetCurrentRotation%20) 90) 360))
      (CallFunction|UpdateConnectionDirs)
      (Utilities|FlowControl|Delay 0.05)
      (Variables|Default|SetbIsRotating false))))

(event Custom|UpdateConnectionDirs)

(event EventInteract
  (params (Interactor :type Actor%20Object%20Reference))
  (bind _caninteract (CallFunction|CanInteract))
  (if _caninteract
    (CallFunction|RotatePipe)
    (bind _returnvalue (Actor|GetActorOfClass "/Game/Bloodlust/Puzzles/Bloodflow/BP_BloodflowManager.BP_BloodflowManager_C"))
    (Default|CheckFlow _returnvalue)))

(fn ConstructionScript)

(fn CanInteract
  (return (not (Variables|Default|GetbIsRotating))))

(fn GetInteractionText
  (return "Rotate"))

(fn SetHighlited
  (params (bIsHighlited :type Boolean)))