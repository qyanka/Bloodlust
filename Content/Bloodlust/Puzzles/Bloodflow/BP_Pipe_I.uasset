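; BP_Pipe_I is a straight pipe piece in the Bloodflow puzzle, connecting two opposite sides.
; On BeginPlay and in its UpdateConnectionDirs event, it sets four directional connection flags from CurrentRotation.
; Rotations that are multiples of 180 open one opposite pair of sides, and any other rotation opens the perpendicular pair.
; The construction script only runs the parent's.
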(event EventBeginPlay
  (CallFunction|UpdateConnectionDirs))

(event EventUpdateConnectionDirs
  (if (== (Math|Integer|%(Integer) (Variables|Default|GetCurrentRotation%20) 180) 0)
    (Variables|Default|SetConnectionDirs (Utilities|Array|MakeArray false true false true))
    (else
      (Variables|Default|SetConnectionDirs (Utilities|Array|MakeArray true false true false)))))

(fn ConstructionScript
  (|CallParentFunction))