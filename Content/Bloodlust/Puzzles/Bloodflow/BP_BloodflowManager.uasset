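; Manager for a bloodflow pipe puzzle that tests whether the source pipe connects to the receiver.
; BeginPlay gathers and logs every BP_PipeBase and refreshes its connection directions.
; CheckFlow runs a breadth-first search capped at 1000 steps, using GetNeighbor and OppositeDir to test connections, and calls PuzzleSolved on reaching the receiver.
; GetNeighbor compares target coordinates to array indices, PuzzleSolved only prints, and HighlightFlow is empty.
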(event Custom|PuzzleSolved
  (Development|PrintString "PuzzleSolved" true true "(R=1.000000,G=0.000000,B=0.021536,A=1.000000)" 1e+01))

(event Custom|HighlightFlow)

(event EventBeginPlay
  (bind _outactors (Actor|GetAllActorsOfClass "/Game/Bloodlust/Puzzles/Bloodflow/BP_PipeBase.BP_PipeBase_C"))
  (bind _output_get (Variables|Default|SetPipeList _outactors))
  (Development|PrintString "PipeList initialized:")
  (for _array_element _output_get
    (Development|PrintString (Utilities|String|Append "Pipe:" (Utilities|GetDisplayName _array_element) " GridX= " (Utilities|String|ToString(Integer) (Variables|/Game/Bloodlust/Puzzles/Bloodflow/BP_PipeBase.BP_PipeBase_C|GetGridX _array_element)) "" " GridY= " (Utilities|String|ToString(Integer) (Variables|/Game/Bloodlust/Puzzles/Bloodflow/BP_PipeBase.BP_PipeBase_C|GetGridY _array_element)) " IsSource " (Utilities|String|ToString(Boolean) (Variables|/Game/Bloodlust/Puzzles/Bloodflow/BP_PipeBase.BP_PipeBase_C|GetbIsSource _array_element)) " IsReceiver " (Utilities|String|ToString(Boolean) (Variables|/Game/Bloodlust/Puzzles/Bloodflow/BP_PipeBase.BP_PipeBase_C|GetbIsReceiver%20 _array_element))))
    (Default|UpdateConnectionDirs _array_element)))

(fn ConstructionScript)

(fn GetNeighbor
  (params (CurrentPipe :type BP%20Pipe%20Base%20Object%20Reference) (Direction :type Integer))
  (bind _gridx (Variables|/Game/Bloodlust/Puzzles/Bloodflow/BP_PipeBase.BP_PipeBase_C|GetGridX CurrentPipe))
  (bind _gridy (Variables|/Game/Bloodlust/Puzzles/Bloodflow/BP_PipeBase.BP_PipeBase_C|GetGridY CurrentPipe))
  (LocalVariables|SetCurrentNeighborX (Variables|/Game/Bloodlust/Puzzles/Bloodflow/BP_PipeBase.BP_PipeBase_C|GetGridX CurrentPipe))
  (LocalVariables|SetCurrentNeighborY (Variables|/Game/Bloodlust/Puzzles/Bloodflow/BP_PipeBase.BP_PipeBase_C|GetGridY CurrentPipe))
  (switch int Direction
    (:0
      (LocalVariables|SetCurrentNeighborY (+ _gridy 1)))
    (:1
      (LocalVariables|SetCurrentNeighborX (+ _gridx 1)))
    (:2
      (LocalVariables|SetCurrentNeighborY (- _gridy 1)))
    (:3
      (LocalVariables|SetCurrentNeighborX (- _gridx 1))))
  (for (_array_element _array_index) (Variables|Default|GetPipeList)
    (if (and (== _array_index (LocalVariables|GetCurrentNeighborY)) (== _array_index (LocalVariables|GetCurrentNeighborX)))
      (return _array_element)
      (else
        (return 0)))))

(fn CheckFlow
  (for _array_element (Variables|Default|GetPipeList)
    (Utilities|FlowControl|Sequence
      (:then_0
        (if (Variables|/Game/Bloodlust/Puzzles/Bloodflow/BP_PipeBase.BP_PipeBase_C|GetbIsSource _array_element)
          (bind _output_get (LocalVariables|SetSourcePipe _array_element))))
      (:then_1
        (if (Variables|/Game/Bloodlust/Puzzles/Bloodflow/BP_PipeBase.BP_PipeBase_C|GetbIsReceiver%20 _array_element)
          (LocalVariables|SetRecieverPipe _array_element)))))
  (LocalVariables|SetVisited (Utilities|Array|MakeArray 0))
  (LocalVariables|SetOpenSet (Utilities|Array|MakeArray 0))
  (bind _output_get_2 (LocalVariables|SetOpenSet (Utilities|Array|MakeArray _output_get)))
  (while (and (> (Utilities|Array|Length _output_get_2) 0) (< (LocalVariables|GetLoopCount) 1000)) :!label _label
    (bind _output_get_3 (LocalVariables|SetCurrentPipe (Utilities|Array|Get(acopy) (LocalVariables|GetOpenSet))))
    (Utilities|Array|RemoveIndex (LocalVariables|GetOpenSet))
    (Math|Integer|IncrementInt (LocalVariables|GetLoopCount)
      (:%20%20
        (if (Utilities|Array|ContainsItem (LocalVariables|GetVisited) _output_get_3)
          (goto _label)
          (else
            (CallFunction|HighlightFlow)
            (Utilities|Array|Add (LocalVariables|GetVisited) (LocalVariables|GetCurrentPipe))
            (if (== (LocalVariables|GetCurrentPipe) (LocalVariables|GetRecieverPipe))
              (CallFunction|PuzzleSolved)
              (else
                (for _index (range 0 3)
                  (if (Utilities|Array|Get(acopy) (Variables|/Game/Bloodlust/Puzzles/Bloodflow/BP_PipeBase.BP_PipeBase_C|GetConnectionDirs (LocalVariables|GetCurrentPipe)) _index)
                    (bind _neighborpipe (CallFunction|GetNeighbor (LocalVariables|GetCurrentPipe) _index))
                    (if (Utilities|IsValid _neighborpipe)
                      (bind _neighborpipe_2 (CallFunction|GetNeighbor (LocalVariables|GetCurrentPipe) _index))
                      (bind _opposite (CallFunction|OppositeDir (Math|Conversions|ToInteger(Boolean) (Utilities|Array|Get(acopy) (Variables|/Game/Bloodlust/Puzzles/Bloodflow/BP_PipeBase.BP_PipeBase_C|GetConnectionDirs _neighborpipe_2) _index))))
                      (if (and (Utilities|Array|Get(acopy) (Variables|/Game/Bloodlust/Puzzles/Bloodflow/BP_PipeBase.BP_PipeBase_C|GetConnectionDirs (LocalVariables|GetCurrentPipe)) _index) (Utilities|Array|Get(acopy) (Variables|/Game/Bloodlust/Puzzles/Bloodflow/BP_PipeBase.BP_PipeBase_C|GetConnectionDirs _neighborpipe_2) _opposite))
                        (bind _neighborpipe_3 (CallFunction|GetNeighbor (LocalVariables|GetCurrentPipe) _index))
                        (if (not (and (Utilities|Array|ContainsItem (LocalVariables|GetVisited) _neighborpipe_3) (Utilities|Array|ContainsItem (LocalVariables|GetOpenSet) _neighborpipe_3)))
                          (Utilities|Array|Add (LocalVariables|GetOpenSet) _neighborpipe_3))))))))))))))

(fn OppositeDir
  (params (Dir :type Integer))
  (switch int Dir
    (:0
      (return 2))
    (:1
      (return 3))
    (:2
      (return 0))
    (:3
      (return 1))))