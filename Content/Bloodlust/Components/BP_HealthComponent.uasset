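; Health component that tracks its owner's health and death state in Bloodlust.
; TakeDamage and IncreaseHealth adjust CurrentHealth within a fixed clamped range, but only damage broadcasts OnHealthChanged.
; Damage that empties health fires OnDied without setting IsDead, whereas Die sets that flag, which blocks further damage, and fires OnDied once.
; The AutoKillOnZeroHP branch in Die is empty.
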(event Custom|TakeDamage
  (params (DamageAmount :type Float%20%28double-precision%29))
  (if (not (Variables|Default|GetbIsDead	))
    (bind _output_get (Variables|Default|SetCurrentHealth (Math|Float|Clamp(Float) (- (Variables|Default|GetCurrentHealth) DamageAmount) 0.0 1e+02)))
    (Default|CallOnHealthChanged _output_get)
    (if (<= _output_get 0.0)
      (Default|CallOnDied))))

(event Custom|Die
  (if (not (Variables|Default|GetbIsDead	))
    (Variables|Default|SetbIsDead	 true)
    (Default|CallOnDied)
    (if (Variables|Default|GetbAutoKillOnZeroHP)
      _)))

(event Custom|IncreaseHealth
  (params (HealthIcreasedValue :type Float%20%28double-precision%29))
  (Variables|Default|SetCurrentHealth (Math|Float|Clamp(Float) (+ HealthIcreasedValue (Variables|Default|GetCurrentHealth)) 0.0 1e+02)))