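; BP_NoiseComponent lets the owning player character emit gameplay noise at a given location.
; Its Noise function looks up the passed name in DT_NoiseData, prints the action name for debugging, and calls PawnMakeNoise with that row's loudness.
; The cooldown gate compares current game time to NoiseCooldown, not time since the last emit, so it only blocks noise early in play.
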(event EventBeginPlay)

(event EventTick
  (params (DeltaSeconds :type Float%20%28single-precision%29)))

(fn Noise
  (params (ActorName :type Name) (Location :type Vector))
  (bind _returnvalue (Components|GetOwner))
  (bind _output_get (Variables|Default|SetLastEmitTime%20 (Utilities|Time|GetTimeSeconds)))
  (if (> _output_get (Variables|Default|GetNoiseCooldown%20))
    (bind _returnvalue_2 (Utilities|GetDataTableRow "/Game/Bloodlust/Data/DT_NoiseData.DT_NoiseData" ActorName)
      (:then
        (bind _asbp_player_character (Utilities|Casting|CastToBP_PlayerCharacter _returnvalue))
        (Development|PrintString (Utilities|String|ToString(Name) (.ActionName (Utilities|Struct|BreakS_NoiseData _returnvalue_2))) true true "(R=0.085650,G=0.333333,B=0.000000,A=1.000000)" 2.0 (.ActionName (Utilities|Struct|BreakS_NoiseData _returnvalue_2)))
        (Class|Pawn|PawnMakeNoise _asbp_player_character (.Loudness (Utilities|Struct|BreakS_NoiseData _returnvalue_2)) Location true _returnvalue))
      (:RowNotFound
        (Development|PrintString "row not found")))))